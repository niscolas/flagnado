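; Flagnado game state that exposes team data to the UI through a global MVVM viewmodel.
; The construction script creates a VM_TeamsData instance if none is valid and registers it in the MVVM game subsystem's global collection.
; On BeginPlay it binds to the team-data-changed delegate and refreshes once, copying GetTeamsData into the viewmodel on each change.
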(event `self.ReceiveBeginPlay`
  (add `self.AnyTeamDataChanged` (`|CreateDelegate` :!event `OnAnyTeamDataChanged`))
  (`self.OnAnyTeamDataChanged`))

(event `OnAnyTeamDataChanged`
  (set `/Game/_Flagnado/UI/VM_TeamsData.AllTeamData` (`self.GetTeamsData`) (`self.VM_TeamsData`)))

(fn `InitGlobalTeamBaseViewmodel`
  (`self.VM_TeamsData`
    (:`then`
      _)
    (:`else`
      (bind _returnvalue (`|GenericCreateObject` "/Game/_Flagnado/UI/VM_TeamsData.VM_TeamsData_C"))
      (set `self.VM_TeamsData` _returnvalue)))
  (`MVVMViewModelCollectionObject.AddViewModelInstance` (`MVVMGameSubsystem.GetViewModelCollection` (subsystem `MVVMGameSubsystem`)) (make `MVVMViewModelContext` "/Game/_Flagnado/UI/VM_TeamsData.VM_TeamsData_C" "VM_TeamsData") (`self.VM_TeamsData`)))

(fn `UserConstructionScript`
  (`self.InitGlobalTeamBaseViewmodel`))