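; Player character for Flagnado, a team flag game, that creates the HUD and feeds team and flag-holding data into a teams viewmodel.
; BeginPlay initializes the viewmodel and adds the UI widget to the viewport.
; Possession on authority and player state updates trigger a client update, which waits briefly before copying team name, color and flag status.
; Flag holder component changes are relayed to the client to update the viewmodel.
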(event `self.ReceiveBeginPlay`
  (bind _viewmodel (`/Game/_Flagnado/Libraries/FunctionLibraries/BPFL_Misc.InitTeamsDataViewmodel`))
  (set `self.VM_TeamsData` _viewmodel)
  (`self.CreateUI`))

(event `self.ReceivePossessed`
  (params (NewController :type "Controller Object Reference"))
  (`/Engine/EditorBlueprintResources/ActorMacros.Switch Has Authority`
    (:`Authority`
      (`self.Client_UpdateViewmodel`))))

(event `Server_OnPlayerStateUpdated`
  (`self.Client_UpdateViewmodel`))

(event `Client_UpdateViewmodel`
  (`KismetSystemLibrary.Delay` 1.0)
  (bind _asflagnado_player_state (cast `FlagnadoPlayerState` (`self.PlayerState`)))
  (set `self.FlagnadoPlayerState` _asflagnado_player_state)
  (`|ExecutionSequence`
    (:`then_0`
      (set `/Game/_Flagnado/UI/VM_TeamsData.CurrentTeamName` (`self.GetCurrentTeamName`) (`self.VM_TeamsData`)))
    (:`then_1`
      (set `/Game/_Flagnado/UI/VM_TeamsData.CurrentTeamColor` (`self.Get Current Team Color`) (`self.VM_TeamsData`)))
    (:`then_2`
      (set `/Game/_Flagnado/UI/VM_TeamsData.IsHoldingTheFlag` (`FlagHolderComponent.CheckIsHoldingTheFlag` (`self.FlagHolderComponent`)) (`self.VM_TeamsData`)))))

(event `self.FlagHolderComponent.IsHoldingTheFlagChanged`
  (params (NewValue :type Boolean))
  (`self.Client_OnIsHoldingTheFlagChanged` NewValue))

(event `Client_OnIsHoldingTheFlagChanged`
  (params (NewParam :type Boolean))
  (set `/Game/_Flagnado/UI/VM_TeamsData.IsHoldingTheFlag` NewParam (`self.VM_TeamsData`)))

(fn `CreateUI`
  (bind _returnvalue (`|CreateWidget` "/Game/_Flagnado/UI/WBP_UI.WBP_UI_C" (cast `PlayerController` (`self.GetController`) :!pure true)))
  (`UserWidget.AddToViewport` _returnvalue 0))

(fn `Get Current Team Color`
  (returns (ReturnValue :type "Color Structure"))
  (return (`TeamsColorProfileDataAsset.GetColorForTeam` (`self.TeamsColorProfileDataAsset`) (`FlagnadoPlayerState.CurrentTeam` (`self.FlagnadoPlayerState`)))))

(fn `GetCurrentTeamName`
  (returns (ReturnValue :type String))
  (return (`|GetEnumeratorNameAsString` (`FlagnadoPlayerState.CurrentTeam` (`self.FlagnadoPlayerState`)))))

(fn `UserConstructionScript`
  (add `self.PlayerStateUpdated` (`|CreateDelegate` :!event `Server_OnPlayerStateUpdated`)))